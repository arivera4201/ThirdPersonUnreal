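; Helper robot NPC that floats in place and shows dialogue text when the player interacts with it.
; Two timelines alternate endlessly to bob and slightly roll the RobotEnemy component.
; Overlap with PlayerCharacter_BP toggles the interaction prompt, and leaving also hides the text box.
; Interact swaps the prompt for a Text_Widget text box and lerps the actor's yaw toward the player, adjusting out-of-range angles.
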(event Custom|Interact
  (Rendering|SetVisibility (Variables|Default|GetTextBox) true false)
  (Rendering|SetVisibility (Variables|Default|GetPromptWidget) false false)
  (Variables|Default|SetLookAtRot (- (.yaw (Math|Rotator|FindLookatRotation (Transformation|GetActorLocation) (Transformation|GetActorLocation (Game|GetPlayerCharacter 0)))) 9e+01))
  (Variables|Default|SetActorRot (.yaw (Transformation|GetActorRotation)))
  (if (> (Math|Float|Absolute(Float) (Variables|Default|GetLookAtRot)) 1.8e+02)
    (Variables|Default|SetLookAtRot (+ (Variables|Default|GetLookAtRot) 3.6e+02))
    (bind _newtrack_0 (Timeline|LookAt_Timeline PlayFromStart)
      (:Update
        (Transformation|SetActorRotation (Math|Rotator|MakeRotator 0.0 0.0 (Math|Float|Lerp (Variables|Default|GetActorRot) (Variables|Default|GetLookAtRot) _newtrack_0)))))
    (else
      (Timeline|LookAt_Timeline PlayFromStart))))

(event EventBeginPlay
  (bind _robotenemy (Variables|Default|GetRobotEnemy))
  (bind _robotenemy_2 (Variables|Default|GetRobotEnemy))
  (bind _returnvalue (UserInterface|CreateWidget "/Game/Blueprints/RobotHelper/Text_Widget.Text_Widget_C" 0 (Variables|Default|GetText)))
  (UserInterface|SetWidget (Variables|Default|GetTextBox) _returnvalue)
  (Components|Timeline|SetPlayRate (Variables|Default|GetMovementTimeline) 0.75)
  (Components|Timeline|SetPlayRate (Variables|Default|GetTimeline_0) 0.75)
  (Variables|Default|SetStartLocation (.z (Variables|/Script/Engine.SceneComponent|GetRelativeLocation (Variables|Default|GetRobotEnemy))))
  (bind _newtrack_0 (Timeline|MovementTimeline PlayFromStart)
    (:Update
      (Transformation|SetRelativeLocation _robotenemy_2 (Math|Vector|MakeVector 0.0 0.0 (Math|Float|Lerp (Variables|Default|GetStartLocation) (- (Variables|Default|GetStartLocation) (Variables|Default|GetOffset)) _newtrack_0)) false false)
      (Transformation|SetRelativeRotation _robotenemy_2 (Math|Rotator|MakeRotator (Math|Float|Lerp 0.0 3.0 _newtrack_0) 0.0 0.0) false false))
    (:Finished
      (bind _newtrack_0_2 (Timeline|Timeline_0 PlayFromStart)
        (:Update
          (Transformation|SetRelativeLocation _robotenemy (Math|Vector|MakeVector 0.0 0.0 (Math|Float|Lerp (- (Variables|Default|GetStartLocation) (Variables|Default|GetOffset)) (Variables|Default|GetStartLocation) _newtrack_0_2)) false false)
          (Transformation|SetRelativeRotation _robotenemy (Math|Rotator|MakeRotator (Math|Float|Lerp 3.0 0.0 _newtrack_0_2) 0.0 0.0) false false))
        (:Finished
          (Timeline|MovementTimeline PlayFromStart))))))

(event Collision|EventActorBeginOverlap
  (params (OtherActor :type Actor%20Object%20Reference))
  (if (== (Utilities|GetClass OtherActor) "/Game/Blueprints/PlayerCharacter_BP.PlayerCharacter_BP_C")
    (Rendering|SetVisibility (Variables|Default|GetPromptWidget) true false)))

(event Collision|EventActorEndOverlap
  (params (OtherActor :type Actor%20Object%20Reference))
  (if (== (Utilities|GetClass OtherActor) "/Game/Blueprints/PlayerCharacter_BP.PlayerCharacter_BP_C")
    (Rendering|SetVisibility (Variables|Default|GetPromptWidget) false false)
    (Rendering|SetVisibility (Variables|Default|GetTextBox) false false)))

(fn ConstructionScript)