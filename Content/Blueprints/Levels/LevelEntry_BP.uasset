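; Level entry trigger actor that loads a numbered level when the player overlaps it, gated on completion of the previous level.
; On overlap by an actor whose class is exactly PlayerCharacter_BP, it reads the LevelsComplete array in Gamestate_BP at index LevelNum - 1.
; If that entry is true it opens the map named "Level_" plus LevelNum; otherwise it only prints a not-complete message.
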(event Collision|EventActorBeginOverlap
  (params (OtherActor :type Actor%20Object%20Reference))
  (if (== (Utilities|GetClass OtherActor) "/Game/Blueprints/PlayerCharacter_BP.PlayerCharacter_BP_C")
    (bind _asgamestate_bp (Utilities|Casting|CastToGamestate_BP (Game|GetGameState)))
    (if (Utilities|Array|Get(acopy) (Variables|/Game/Blueprints/Gamemode/Gamestate_BP.Gamestate_BP_C|GetLevelsComplete _asgamestate_bp) (- (Variables|Default|GetLevelNum) 1))
      (Game|OpenLevel(byName) (Utilities|String|StringToName (Utilities|String|Append "Level_" (Utilities|String|ToString(Integer) (Variables|Default|GetLevelNum)))))
      (else
        (Development|PrintString "PREVIOUS LEVEL NOT COMPLETE")))))

(fn ConstructionScript)