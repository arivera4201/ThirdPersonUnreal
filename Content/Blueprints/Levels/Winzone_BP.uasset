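; Winzone_BP is a level-end trigger that registers a win when the player character overlaps it.
; Once only, it prints a win message, marks its LevelNumber complete in Gamestate_BP and adds a skill point.
; It writes completed levels and collected nuts to a fresh GameData_BP save in the "savedata" slot, without copying skill points.
; After a short delay it opens the Home level.
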(event Collision|EventActorBeginOverlap
  (params (OtherActor :type Actor%20Object%20Reference))
  (if (== (Utilities|GetClass OtherActor) "/Game/Blueprints/PlayerCharacter_BP.PlayerCharacter_BP_C")
    (bind _asplayer_character_bp (Utilities|Casting|CastToPlayerCharacter_BP OtherActor))
    (Utilities|FlowControl|DoOnce false
      (:Completed
        (Development|PrintString "PLAYER WIN")
        (bind _asgamestate_bp (Utilities|Casting|CastToGamestate_BP (Game|GetGameState)))
        (Utilities|Array|SetArrayElem (Variables|/Game/Blueprints/Gamemode/Gamestate_BP.Gamestate_BP_C|GetLevelsComplete _asgamestate_bp) (Variables|Default|GetLevelNumber) true)
        (Math|Integer|IncrementInt (Variables|/Game/Blueprints/Gamemode/Gamestate_BP.Gamestate_BP_C|GetSkillPoints _asgamestate_bp)
          (:%20%20
            (bind _returnvalue (SaveGame|CreateSaveGameObject "/Game/Blueprints/Gamemode/GameData_BP.GameData_BP_C"))
            (Variables|/Game/Blueprints/Gamemode/GameData_BP.GameData_BP_C|SetLevelsComplete _returnvalue (Variables|/Game/Blueprints/Gamemode/Gamestate_BP.Gamestate_BP_C|GetLevelsComplete _asgamestate_bp))
            (Variables|/Game/Blueprints/Gamemode/GameData_BP.GameData_BP_C|SetNutsCollected _returnvalue (Variables|/Game/Blueprints/PlayerCharacter_BP.PlayerCharacter_BP_C|GetNutsCollected _asplayer_character_bp))
            (SaveGame|SaveGametoSlot _returnvalue "savedata")
            (Utilities|FlowControl|Delay 3.0)
            (Game|OpenLevel(byName) "Home")))))))

(fn ConstructionScript)