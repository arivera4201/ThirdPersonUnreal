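; Moving laser hazard that slides its cylinder along an XYZ offset and deals damage to any actor that overlaps it.
; After a start offset delay, two timelines with a play rate of TimeToMove alternately lerp the cylinder's relative location with teleport moves.
; A delay precedes each return leg, while the out delay applies only before the first move because the loop restarts the timeline directly.
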(event Custom|MoveWall
  (Utilities|FlowControl|Delay (Variables|Default|GetDelayToOut))
  (bind _newtrack_0 (Timeline|MoveTime PlayFromStart)
    (:Update
      (Transformation|SetRelativeLocation (Variables|Default|GetCylinder) (Math|Vector|MakeVector (Math|Float|Lerp 0.0 (Variables|Default|GetXMove) _newtrack_0) (Math|Float|Lerp 0.0 (Variables|Default|GetYMove) _newtrack_0) (Math|Float|Lerp 0.0 (Variables|Default|GetZMove) _newtrack_0)) false true))
    (:Finished
      (Utilities|FlowControl|Delay (Variables|Default|GetDelayToIn))
      (bind _newtrack_0_2 (Timeline|Timeline_0 ReverseFromEnd)
        (:Update
          (Transformation|SetRelativeLocation (Variables|Default|GetCylinder) (Math|Vector|MakeVector (Math|Float|Lerp (Variables|Default|GetXMove) 0.0 _newtrack_0_2) (Math|Float|Lerp (Variables|Default|GetYMove) 0.0 _newtrack_0_2) (Math|Float|Lerp (Variables|Default|GetZMove) 0.0 _newtrack_0_2)) false true))
        (:Finished
          (Timeline|MoveTime PlayFromStart))))))

(event EventBeginPlay
  (bind _timetomove (Variables|Default|GetTimeToMove))
  (Components|Timeline|SetPlayRate (Variables|Default|GetMoveTime) _timetomove)
  (Components|Timeline|SetPlayRate (Variables|Default|GetTimeline_0) _timetomove)
  (Utilities|FlowControl|Delay (Variables|Default|GetOffsetTime))
  (CallFunction|MoveWall))

(event Collision|EventActorBeginOverlap
  (params (OtherActor :type Actor%20Object%20Reference))
  (Game|Damage|ApplyDamage OtherActor 1.0 0 0))

(fn ConstructionScript)