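; Player character Blueprint for a robot with camera-relative movement, timeline-driven double jump with switched gravity, montage-only crouch and Helper interaction via sphere trace.
; Throw triggers a three-punch combo using montages and trace damage, while Sprint raises a temporary shield that spends recharging stamina.
; Unshielded hits shake the camera and step health down through face materials, ending in ragdoll death, a fade-in widget and a game-mode restart.
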(event Custom|StaminaRecharge
  (Utilities|FlowControl|Delay (Variables|Default|GetstaminaRechargeTime))
  (Timeline|StaminaCharge PlayFromStart
    (:Update
      (if (or (Variables|Shields|GetShielding) (>= (Variables|Shields|GetcurrentStamina) (Variables|Shields|GetmaxStamina)))
        (if (>= (Variables|Shields|GetcurrentStamina) (Variables|Shields|GetmaxStamina))
          (Variables|Shields|SetcurrentStamina (Variables|Shields|GetmaxStamina))
          (Timeline|StaminaCharge Stop)
          (else
            (Timeline|StaminaCharge Stop)))
        (else
          (Variables|Shields|SetcurrentStamina (+ (Variables|Shields|GetcurrentStamina) (Variables|Default|GetstaminaRechargeRate))))))))

(event Custom|PunchRecharge
  (Timeline|PunchCooldown PlayFromStart
    (:Finished
      (Variables|Default|SetpunchesThrown 0))))

(event Game|Damage|EventAnyDamage
  (params (Damage :type Float%20%28single-precision%29) (DamageType :type Damage%20Type%20Object%20Reference) (InstigatedBy :type Controller%20Object%20Reference) (DamageCauser :type Actor%20Object%20Reference))
  (bind _health (Variables|Default|GetHealth))
  (bind _mesh (Variables|Character|GetMesh))
  (if (not (Variables|Shields|GetShielding))
    (CameraShakes|StartCameraShake (Game|GetPlayerCameraManager 0) "/Game/Blueprints/Damage_Shake.Damage_Shake_C" 1.0 "CameraLocal" "0, 0, 0")
    (switch int (Variables|Default|GetHealth)
      (:1
        (Utilities|FlowControl|DoOnce false
          (:Completed
            (CallFunction|Death)
            (Utilities|FlowControl|Delay (Variables|Default|GetrespawnTime))
            (CallFunction|Respawn))))
      (:2
        (Math|Integer|DecrementInt _health
          (:%20%20
            (Rendering|Material|SetMaterial _mesh 1 "/Game/Models/Robot/Materials/SadFace_Mat.SadFace_Mat"))))
      (:3
        (Math|Integer|DecrementInt _health
          (:%20%20
            (Rendering|Material|SetMaterial _mesh 1 "/Game/Models/Robot/Materials/NeutralFace_Mat.NeutralFace_Mat")))))))

(event EventOnLanded
  (params (Hit :type Hit%20Result%20Structure%20%28by%20ref%29))
  (Variables|Default|SetjumpsLeft (Variables|Default|GetjumpsMax))
  (Animation|Montage|PlayMontage (Variables|Character|GetMesh) "/Game/Models/Robot/Anims/Jump/LandMontage.LandMontage" 1.0 0.0 "Land"
    (:then
      (Variables|Default|SetisGrounded true)
      (Variables|/Script/Engine.CharacterMovementComponent|SetRotationRate (Variables|Character|GetCharacterMovement) (Math|Rotator|MakeRotator 0.0 0.0 (Variables|Default|GetZRotationRate)))
      (Variables|Default|SetCameraInterpSpeed 5e+01))))

(event EventBeginPlay
  ;[1 1 1] BeginPlay
  (Camera|SetFieldOfView (Variables|Default|GetPlayerCamera) (Variables|PlayerSettings|GetPlayerFOV))
  (bind _returnvalue (UserInterface|CreateWidget "/Game/Blueprints/HUD/Combat_Widget.Combat_Widget_C"))
  (bind _output_get (Variables|HUD|SetCombatWidget _returnvalue))
  (UserInterface|Viewport|AddtoViewport _output_get 0)
  (Widget|SetVisibility _output_get "Hidden")
  (bind _returnvalue_2 (UserInterface|CreateWidget "/Game/Blueprints/HUD/HUD_Widget.HUD_Widget_C"))
  (bind _output_get_2 (Variables|HUD|SetPlayerHUD _returnvalue_2))
  (UserInterface|Viewport|AddtoViewport _output_get_2 0)
  (Utilities|FlowControl|Delay 0.01)
  (Class|SkeletalMeshComponent|SetAnimClass (Variables|Character|GetMesh) "/Game/Models/Robot/Robot_Anim_BP.Robot_Anim_BP_C"))

(event EventOnWalkingOffLedge
  (params (PreviousFloorImpactNormal :type Vector%20%28by%20ref%29 :default "0, 0, 0") (PreviousFloorContactNormal :type Vector%20%28by%20ref%29 :default "0, 0, 0") (PreviousLocation :type Vector%20%28by%20ref%29 :default "0, 0, 0") (TimeDelta :type Float%20%28single-precision%29))
  (Math|Integer|DecrementInt (Variables|Default|GetjumpsLeft)
    (:%20%20
      (Variables|Default|SetisGrounded false)
      (Variables|/Script/Engine.CharacterMovementComponent|SetRotationRate (Variables|Character|GetCharacterMovement) (Math|Rotator|MakeRotator 0.0 0.0 25.0))
      (Variables|Default|SetCameraInterpSpeed 3e+01))))

(event Input|ActionEvents|InputActionJump
  (params (Key :type Key%20Structure :default "None"))
  (bind _returnvalue (Transformation|GetVelocity))
  (:Pressed
    (if (>= (Variables|Default|GetjumpsLeft) 1)
      (Variables|/Script/Engine.CharacterMovementComponent|SetRotationRate (Variables|Character|GetCharacterMovement) (Math|Rotator|MakeRotator 0.0 0.0 25.0))
      (Variables|Default|SetCameraInterpSpeed 3e+01)
      (Variables|Default|SetisGrounded false)
      (Variables|/Script/Engine.CharacterMovementComponent|SetGravityScale (Variables|Character|GetCharacterMovement) (Variables|Default|GetJumpGravity))
      (Variables|Default|SetisJumping true)
      (Math|Integer|DecrementInt (Variables|Default|GetjumpsLeft)
        (:%20%20
          (switch int (Variables|Default|GetjumpsLeft)
            (:Default
              (bind _newtrack_0 (Timeline|Jump%20Timeline PlayFromStart)
                (:Update
                  (Character|LaunchCharacter (Math|Vector|MakeVector (* (.x _returnvalue) 0.001) (* (.y _returnvalue) 0.001) (Math|Float|Lerp 0.0 (Variables|Default|GetJumpHeight) _newtrack_0)) false true))
                (:Finished
                  (Variables|/Script/Engine.CharacterMovementComponent|SetGravityScale (Variables|Character|GetCharacterMovement) (Variables|Default|GetFallGravity) :!label _label)
                  (if (Variables|Default|GetisJumping)
                    (Variables|Default|SetisJumping false)))))
            (:0
              (bind _output_get (Variables|Default|SetJumpHeight 1.8e+03))
              (Animation|Montage|PlayMontage (Variables|Character|GetMesh) "/Game/Models/Robot/Anims/Jump/DoubleJumpMontage.DoubleJumpMontage" 1.0 0.0 "Jump"
                (:then
                  (Character|LaunchCharacter (Math|Vector|MakeVector 0.0 0.0 _output_get) false true)
                  (goto _label))))
            (:1
              (Variables|Default|SetJumpHeight 8e+02)
              (Animation|Montage|PlayMontage (Variables|Character|GetMesh) "/Game/Models/Robot/Anims/Jump/NewJumpMontage.NewJumpMontage" 1.0 0.0 "Jump"
                (:then
                  (Timeline|Jump%20Timeline PlayFromStart)))))))))
  (:Released
    (Variables|Default|SetisJumping false)
    (Variables|/Script/Engine.CharacterMovementComponent|SetGravityScale (Variables|Character|GetCharacterMovement) (Variables|Default|GetFallGravity))
    (Timeline|Jump%20Timeline Stop)))

(event Input|ActionEvents|InputActionSprint
  (params (Key :type Key%20Structure :default "None"))
  (:Pressed
    (if (and (not (Variables|Shields|GetShielding)) (> (Variables|Shields|GetcurrentStamina) 0.001))
      (if (>= (Variables|Shields|GetcurrentStamina) (- (/ (Variables|Shields|GetmaxStamina) (Variables|Shields|GetshieldNum)) 0.02))
        (Variables|Shields|SetShielding true :!label _label)
        (Rendering|SetVisibility (Variables|Default|GetSphere) true false)
        (Variables|Shields|SetcurrentStamina (- (Variables|Shields|GetcurrentStamina) (/ (Variables|Shields|GetmaxStamina) (Variables|Shields|GetshieldNum))))
        (Utilities|FlowControl|Delay (Variables|Shields|GetshieldUpTime))
        (Rendering|SetVisibility (Variables|Default|GetSphere) false false)
        (Utilities|FlowControl|Delay (Variables|Shields|GetshieldCooldown))
        (Variables|Shields|SetShielding false)
        (CallFunction|StaminaRecharge)
        (else
          (Utilities|FlowControl|Sequence
            (:then_0
              (goto _label))
            (:then_1
              (Variables|Shields|SetcurrentStamina 0.0)
              (Variables|/Script/Engine.CharacterMovementComponent|SetMaxWalkSpeed (Variables|Character|GetCharacterMovement) (/ (Variables|Default|GetwalkSpeed) 2.0))
              (Utilities|FlowControl|Delay 3.0)
              (Variables|/Script/Engine.CharacterMovementComponent|SetMaxWalkSpeed (Variables|Character|GetCharacterMovement) (Variables|Default|GetwalkSpeed)))))))))

(event Input|ActionEvents|InputActionCrouch
  (params (Key :type Key%20Structure :default "None"))
  (bind _mesh (Variables|Character|GetMesh))
  (:Pressed
    (Animation|Montage|PlayMontage _mesh "/Game/Models/Robot/Anims/Movement/RobotCrouch_Montage.RobotCrouch_Montage" 1.0 0.0 "Crouch"))
  (:Released
    (Animation|Montage|PlayMontage _mesh "/Game/Models/Robot/Anims/Movement/RobotCrouch_Montage.RobotCrouch_Montage" -1.0 0.0 "Crouch")))

(event Input|ActionEvents|InputActionInteract
  (params (Key :type Key%20Structure :default "None"))
  (bind _mesh (Variables|Character|GetMesh))
  (bind _hitobjects (Variables|Default|GetHitObjects))
  (bind _returnvalue (Transformation|GetWorldLocation _mesh))
  (:Pressed
    (Development|PrintString (Utilities|String|ToString(Integer) (Variables|Default|GetNutsCollected)))
    (bind _outhits (Collision|MultiSphereTraceByChannel _returnvalue _returnvalue 249.5 "TraceTypeQuery1" false 0 "None"))
    (bind _array_element (Utilities|Array|ForEachLoopwithBreak _outhits)
      (:LoopBody
        (if (not (> (Utilities|Array|FindItem _hitobjects (.HitActor (Collision|BreakHitResult _array_element))) -1))
          (if true
            (Utilities|Array|Add _hitobjects (.HitActor (Collision|BreakHitResult _array_element)))
            (if (== (Utilities|GetClass (.HitActor (Collision|BreakHitResult _array_element))) "/Game/Blueprints/RobotHelper/Helper_BP.Helper_BP_C")
              (bind _ashelper_bp (Utilities|Casting|CastToHelper_BP (.HitActor (Collision|BreakHitResult _array_element))))
              (Default|Interact _ashelper_bp)))))
      (:Completed
        (Utilities|Array|Clear (Variables|Default|GetHitObjects))))))

(event Input|ActionEvents|InputActionThrow
  (params (Key :type Key%20Structure :default "None"))
  (bind _capsulecomponent (Variables|Collision|GetCapsuleComponent))
  (bind _returnvalue (Transformation|GetWorldLocation _capsulecomponent))
  (bind _returnvalue_2 (Math|Vector|GetForwardVector _capsulecomponent))
  (:Pressed
    (if (and (Variables|Default|GetcanPunch) (< (Variables|Default|GetpunchesThrown) 3))
      (Math|Integer|IncrementInt (Variables|Default|GetpunchesThrown)
        (:%20%20
          (Variables|Default|SetcanPunch false)
          ;[1 1 1] Combat
          ;;[1 1 1] PlayPunchAnim
          (Animation|Montage|PlayMontage (Variables|Character|GetMesh) (Utilities|Array|Get(acopy) (Variables|Default|GetAttackAnims) (- (Variables|Default|GetpunchesThrown) 1)) 1.0 0.0 "Attack"
            (:then
              (Utilities|FlowControl|Delay (Variables|Default|GetTimeToPunch))
              (bind _outhit (Collision|SphereTraceByChannel (+ _returnvalue (* _returnvalue_2 5e+01)) (+ _returnvalue (* _returnvalue_2 1.5e+02)) 75.0 "TraceTypeQuery1" false 0 "None"))
              (Game|Damage|ApplyDamage (.HitActor (Collision|BreakHitResult _outhit)) 1e+01 0 0)
              (Utilities|FlowControl|Delay (* (Variables|Default|GetTimeToPunch) 2.0))
              (Variables|Default|SetcanPunch true)
              (CallFunction|PunchRecharge))))))))

(event Input|AxisEvents|InputAxisMouseHorizontal
  (params (AxisValue :type Float%20%28single-precision%29))
  ;[1 1 1] Look & Movement
  (Pawn|Input|AddControllerYawInput (* AxisValue (Variables|PlayerSettings|GetPlayerSens)))
  (if (or (!= AxisValue 0.0) (!= (stale Input|AxisEvents|InputAxisMouseVertical AxisValue) 0.0))
    (Variables|Default|SetCameraStill false)
    (Timeline|Timeline_0 PlayFromStart
      (:Finished
        (Variables|Default|SetCameraStill true)))
    (else
      (Timeline|Timeline_0 Play))))

(event Input|AxisEvents|InputAxisMouseVertical
  (params (AxisValue :type Float%20%28single-precision%29))
  ;[1 1 1] Look & Movement
  (Pawn|Input|AddControllerPitchInput (* AxisValue (Variables|PlayerSettings|GetPlayerSens)))
  (if (or (!= (stale Input|AxisEvents|InputAxisMouseHorizontal AxisValue) 0.0) (!= AxisValue 0.0))
    (Variables|Default|SetCameraStill false)
    (Timeline|Timeline_0 PlayFromStart
      (:Finished
        (Variables|Default|SetCameraStill true)))
    (else
      (Timeline|Timeline_0 Play))))

(event Input|AxisEvents|InputAxisVertical
  (params (AxisValue :type Float%20%28single-precision%29))
  (bind _returnvalue (Pawn|GetController))
  (bind _returnvalue_2 (Pawn|GetControlRotation _returnvalue :!class /Script/Engine.Controller))
  ;[1 1 1] Look & Movement
  (Pawn|Input|AddMovementInput (Math|Vector|GetForwardVector (Pawn|GetControlRotation :!class /Script/Engine.Pawn)) AxisValue false)
  (if (and (or (!= AxisValue 0.0) (!= (stale Input|AxisEvents|InputAxisHorizontal AxisValue) 0.0)) (Variables|Default|GetCameraStill))
    (Pawn|SetControlRotation _returnvalue (Math|Rotator|MakeRotator (.roll _returnvalue_2) (.pitch _returnvalue_2) (Math|Interpolation|FInterpTo (.yaw _returnvalue_2) (+ (stale Input|AxisEvents|InputAxisHorizontal AxisValue) (.yaw _returnvalue_2)) (Utilities|Time|GetWorldDeltaSeconds) (Variables|Default|GetCameraInterpSpeed))))))

(event Input|AxisEvents|InputAxisHorizontal
  (params (AxisValue :type Float%20%28single-precision%29))
  (bind _returnvalue (Pawn|GetController))
  (bind _returnvalue_2 (Pawn|GetControlRotation _returnvalue :!class /Script/Engine.Controller))
  ;[1 1 1] Look & Movement
  (Pawn|Input|AddMovementInput (Math|Vector|GetRightVector (Pawn|GetControlRotation :!class /Script/Engine.Pawn)) AxisValue false)
  (if (and (or (!= (stale Input|AxisEvents|InputAxisVertical AxisValue) 0.0) (!= AxisValue 0.0)) (Variables|Default|GetCameraStill))
    (Pawn|SetControlRotation _returnvalue (Math|Rotator|MakeRotator (.roll _returnvalue_2) (.pitch _returnvalue_2) (Math|Interpolation|FInterpTo (.yaw _returnvalue_2) (+ AxisValue (.yaw _returnvalue_2)) (Utilities|Time|GetWorldDeltaSeconds) (Variables|Default|GetCameraInterpSpeed))))))

(fn ConstructionScript)

(fn Death
  (bind _mesh (Variables|Character|GetMesh))
  (Collision|SetCollisionEnabled _mesh "PhysicsOnly")
  (Physics|SetSimulatePhysics _mesh true)
  (Variables|/Script/Engine.CharacterMovementComponent|SetMaxWalkSpeed (Variables|Character|GetCharacterMovement) 0.0)
  (bind _returnvalue (UserInterface|CreateWidget "/Game/Blueprints/HUD/Death_Widget.Death_Widget_C"))
  (UserInterface|Viewport|AddtoViewport _returnvalue 0)
  (UserInterface|Animation|PlayAnimation _returnvalue (Variables|/Game/Blueprints/HUD/Death_Widget.Death_Widget_C|GetFadeIn _returnvalue) 0.0 1 "Forward" 1.0 false))

(fn Respawn
  (bind _asplayer_gamemode_bp (Utilities|Casting|CastToPlayer_Gamemode_BP (Game|GetGameMode)))
  (Class|GameMode|RestartGame _asplayer_gamemode_bp))