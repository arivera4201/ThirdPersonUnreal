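; Treadmill actor that pushes the player along the forward direction of its Cube component while they overlap it.
; Begin overlap sets a touching flag and starts a short Delay loop that repeatedly calls LaunchCharacter, adding velocity until end overlap clears the flag.
; The flag changes for any overlapping actor, though only PlayerCharacter_BP is launched.
; An unconnected branch that doubles walk speed never runs.
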(event Collision|EventActorBeginOverlap
  (params (OtherActor :type Actor%20Object%20Reference))
  (Variables|Default|SettouchingPlayer true)
  (bind _asplayer_character_bp (Utilities|Casting|CastToPlayerCharacter_BP OtherActor))
  (if (Variables|Default|GettouchingPlayer) :!label _label
    (Character|LaunchCharacter _asplayer_character_bp (* (Math|Vector|GetForwardVector (Variables|Default|GetCube)) 1.1e+02) false false)
    (Utilities|FlowControl|Delay 0.05)
    (goto _label)))

(event Collision|EventActorEndOverlap
  (params (OtherActor :type Actor%20Object%20Reference))
  (Variables|Default|SettouchingPlayer false))

(fn ConstructionScript)